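; BP_Charger is an NPC character that takes damage from the player's sword and dies when health runs out.
; Capsule overlaps with BP_Sword subtract its damage only during the player's fast attack and while hittable, printing health for debugging.
; Surviving hits trigger brief immunity through a delay.
; Lethal hits set IsDead on the AI controller's blackboard, then destroy the actor after a delay.
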(event `self.CapsuleComponent.OnComponentBeginOverlap`
  (params (OverlappedComponent :type "PrimitiveComponent Object Reference") (OtherActor :type "Actor Object Reference") (OtherComp :type "PrimitiveComponent Object Reference") (OtherBodyIndex :type Integer) (bFromSweep :type Boolean) (SweepResult :type "HitResult Structure (by ref)"))
  ;[1 1 1] Getting damage from sword heats
  (bind _asbp_sword (cast `/Game/Weapons/Blueprints/BP_Sword` OtherActor))
  (bind _asbp_sword_character (cast `/Game/Characters/Player/Blueprints/BP_SwordCharacter` (`GameplayStatics.GetPlayerCharacter` 0)))
  (if (`/Game/Characters/Player/Blueprints/BP_SwordCharacter.FastSwordAttack` _asbp_sword_character)
    (if (`self.CanBeHit`)
      (bind _output_get (set `self.Health` (- (`self.Health`) (`/Game/Weapons/Blueprints/BP_Sword.Damage` _asbp_sword))))
      (`|ExecutionSequence`
        (:`then_0`
          ;[1 1 1] Checking death
          (if (<= _output_get 0.0)
            (bind _output_get_2 (set `self.IsDead` true))
            (`|ExecutionSequence`
              (:`then_0`
                (`BlackboardComponent.SetValueAsBool` (`AIBlueprintHelperLibrary.GetBlackboard` (`AIBlueprintHelperLibrary.GetAIController` self)) "IsDead" _output_get_2))
              (:`then_1`
                (`KismetSystemLibrary.Delay` 2.8)
                (`self.Death`)))
            (else
              ;[1 1 1] Temp immunity after hit
              (set `self.CanBeHit` false)
              (`KismetSystemLibrary.Delay` 1.0)
              (set `self.CanBeHit` true))))
        (:`then_1`
          (`KismetSystemLibrary.PrintString` (`KismetStringLibrary.Conv_DoubleToString` _output_get) true true (struct :`R` 1.0 :`G` 0.045875 :`A` 1.0)))))))

(fn `Death`
  (`self.K2_DestroyActor`))

(fn `UserConstructionScript`)