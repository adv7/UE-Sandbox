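; BP_AITest is a test NPC that takes sword damage from the player and is destroyed when its health runs out.
; A capsule overlap with a BP_Sword subtracts the sword's damage from Health, but only while the player character's FastSwordAttack flag is set.
; At zero health or below it sets IsDead and calls Death, which destroys the actor.
; The file contains no movement or decision-making logic.
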(event `self.CapsuleComponent.OnComponentBeginOverlap`
  (params (OverlappedComponent :type "PrimitiveComponent Object Reference") (OtherActor :type "Actor Object Reference") (OtherComp :type "PrimitiveComponent Object Reference") (OtherBodyIndex :type Integer) (bFromSweep :type Boolean) (SweepResult :type "HitResult Structure (by ref)"))
  ;[1 1 1] Getting damage from sword heats
  (bind _asbp_sword (cast `/Game/Weapons/Blueprints/BP_Sword` OtherActor))
  (bind _asbp_sword_character (cast `/Game/Characters/Player/Blueprints/BP_SwordCharacter` (`GameplayStatics.GetPlayerCharacter` 0)))
  (if (`/Game/Characters/Player/Blueprints/BP_SwordCharacter.FastSwordAttack` _asbp_sword_character)
    (bind _output_get (set `self.Health` (- (`self.Health`) (`/Game/Weapons/Blueprints/BP_Sword.Damage` _asbp_sword))))
    ;[1 1 1] Checking death
    (if (<= _output_get 0.0)
      (set `self.IsDead` true)
      (`self.Death`))))

(fn `Death`
  (`self.K2_DestroyActor`))

(fn `UserConstructionScript`)